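; BP_Julie is a top-down pawn that hides static meshes between its camera and capsule.
; Each tick it reapplies stored materials, clears its lists, then runs a debug-drawn multi capsule trace and swaps hit meshes to M_Invisible.
; The restore uses nested loops and the array index as material slot, so materials are not paired per mesh.
; Space hides the character mesh; confetti and visibility-restore snippets are unconnected.
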(event `self.ReceiveTick`
  (params (DeltaSeconds :type "Float (single-precision)"))
  (bind _elementinvisible (`self.ElementInvisible`))
  (bind _elementinvisible_2 (`self.ElementInvisible`))
  (bind _materialinvisible (`self.MaterialInvisible`))
  (for (_array_element _array_index) _elementinvisible_2
    (for _array_element_2 _materialinvisible
      (`PrimitiveComponent.SetMaterial` _array_element _array_index _array_element_2)))
  (`KismetArrayLibrary.Array_Clear` _materialinvisible)
  (`KismetArrayLibrary.Array_Clear` _elementinvisible_2)
  (bind _outhits (`KismetSystemLibrary.CapsuleTraceMulti` :`Start` (`SceneComponent.K2_GetComponentLocation` (`self.TopDownCameraComponent`)) :`End` (`SceneComponent.RelativeLocation` (`self.CapsuleComponent`)) :`Radius` 1.0 :`TraceChannel` "TraceTypeQuery1" :`DrawDebugType` "ForDuration" :`DrawTime` 2.0))
  (for _array_element_3 _outhits
    (bind _asstatic_mesh_component (cast `StaticMeshComponent` (`.HitComponent` (`GameplayStatics.BreakHitResult` _array_element_3))))
    (`KismetArrayLibrary.Array_Add` (`self.MaterialInvisible`) (`PrimitiveComponent.GetMaterial` _asstatic_mesh_component 0))
    (`KismetArrayLibrary.Array_Add` _elementinvisible _asstatic_mesh_component)
    (for _array_element_4 _elementinvisible
      (`PrimitiveComponent.SetMaterial` _array_element_4 0 "/Game/GA_asset/M_Invisible.M_Invisible"))))

(event `Key|SpaceBar`
  (params (Key :type "Key Structure"))
  (:`Pressed`
    (`SceneComponent.SetVisibility` (`self.Mesh`) false true)))

(fn `UserConstructionScript`)